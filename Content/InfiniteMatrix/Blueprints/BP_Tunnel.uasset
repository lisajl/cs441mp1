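; BP_Tunnel is a tunnel segment for an endless runner, with a rotating wall obstacle.
; Reaching the trigger zone raises player speed and score, has TunnelSpawner spawn another segment, then destroys this one.
; Touching the wall costs health, showing restart at zero, and leaving it costs score.
; Helper functions randomize the hole mesh and roll, and pick the material from a randomly seeded, incrementable counter.
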(event OnComponentBeginOverlap(TriggerZone)
  (params (OverlappedComponent :type Primitive%20Component%20Object%20Reference) (OtherActor :type Actor%20Object%20Reference) (OtherComp :type Primitive%20Component%20Object%20Reference) (OtherBodyIndex :type Integer) (bFromSweep :type Boolean) (SweepResult :type Hit%20Result%20Structure%20%28by%20ref%29))
  (bind _asbp_player (Utilities|Casting|CastToBP_Player OtherActor))
  (Variables|/Game/InfiniteMatrix/Blueprints/BP_Player.BP_Player_C|SetForwardSpeed _asbp_player (+ (Variables|/Game/InfiniteMatrix/Blueprints/BP_Player.BP_Player_C|GetForwardSpeed _asbp_player) 4e+01))
  (Default|AddScore _asbp_player)
  (Default|SpawnTunnelatSpawnPoint (Variables|Default|GetTunnelSpawner))
  (Actor|DestroyActor))

(event OnComponentEndOverlap(WallMesh)
  (params (OverlappedComponent :type Primitive%20Component%20Object%20Reference) (OtherActor :type Actor%20Object%20Reference) (OtherComp :type Primitive%20Component%20Object%20Reference) (OtherBodyIndex :type Integer))
  (bind _asbp_player (Utilities|Casting|CastToBP_Player OtherActor))
  (Default|LoseScore _asbp_player))

(event OnComponentBeginOverlap(WallMesh)
  (params (OverlappedComponent :type Primitive%20Component%20Object%20Reference) (OtherActor :type Actor%20Object%20Reference) (OtherComp :type Primitive%20Component%20Object%20Reference) (OtherBodyIndex :type Integer) (bFromSweep :type Boolean) (SweepResult :type Hit%20Result%20Structure%20%28by%20ref%29))
  (bind _asbp_player (Utilities|Casting|CastToBP_Player OtherActor))
  (Default|LoseHealth _asbp_player)
  (if (== (Variables|/Game/InfiniteMatrix/Blueprints/BP_Player.BP_Player_C|GetHealth _asbp_player) 0.0)
    (Default|DisplayRestart _asbp_player)))

(event EventBeginPlay
  (Variables|Default|SetMeshCounter (Math|Random|RandomIntegerinRange 0 7)))

(event EventTick
  (params (DeltaSeconds :type Float%20%28single-precision%29))
  (Transformation|AddLocalRotation (Variables|Default|GetWallMesh) (Math|Rotator|MakeRotator (* DeltaSeconds (Variables|Default|GetRotateSpeed)) 0.0 0.0) false false))

(fn ConstructionScript)

(fn RandomizeWall
  (Components|StaticMesh|SetStaticMesh (Variables|Default|GetWallMesh) (Utilities|Select :Index (Math|Random|RandomIntegerinRange 0 3) :Option%200 "/Game/InfiniteMatrix/Meshes/SM_Hole_01.SM_Hole_01" :Option%201 "/Game/InfiniteMatrix/Meshes/SM_Hole_02.SM_Hole_02" :Option%202 "/Game/InfiniteMatrix/Meshes/SM_Hole_03.SM_Hole_03" :Option%203 "/Game/InfiniteMatrix/Meshes/SM_Hole_04.SM_Hole_04"))
  (Transformation|AddLocalRotation (Variables|Default|GetWallMesh) (Math|Rotator|MakeRotator (Math|Random|RandomFloatinRange 0.0 3.6e+02) 0.0 0.0) false false))

(fn WallMaterial
  (Rendering|Material|SetMaterial (Variables|Debug|GetStaticMeshComponent) 0 (Utilities|Select :Index (Math|Integer|%(Integer) (Variables|Default|GetMeshCounter) 8) :Option%200 "/Game/InfiniteMatrix/Materials/blue.blue" :Option%201 "/Game/InfiniteMatrix/Materials/darkblue.darkblue" :Option%202 "/Game/InfiniteMatrix/Materials/purple.purple" :Option%203 "/Game/InfiniteMatrix/Materials/pink.pink" :Option%204 "/Game/InfiniteMatrix/Materials/red.red" :Option%205 "/Game/InfiniteMatrix/Materials/orange.orange" :Option%206 "/Game/InfiniteMatrix/Materials/darkblue3.darkblue3" :Option%207 "/Game/InfiniteMatrix/Materials/green.green")))

(fn MeshAdd
  (Variables|Default|SetMeshCounter (+ (Variables|Default|GetMeshCounter) 1)))