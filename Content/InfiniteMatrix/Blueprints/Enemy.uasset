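; Enemy actor that spins around its roll axis every tick and reacts to overlaps on its Cube2 component.
; Touching BP_Player makes the player lose health, destroys the enemy, and shows the restart screen when health reaches zero.
; Being hit by a Projectile destroys the enemy and adds score to the player pawn.
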(event OnComponentBeginOverlap(Cube2)
  (params (OverlappedComponent :type Primitive%20Component%20Object%20Reference) (OtherActor :type Actor%20Object%20Reference) (OtherComp :type Primitive%20Component%20Object%20Reference) (OtherBodyIndex :type Integer) (bFromSweep :type Boolean) (SweepResult :type Hit%20Result%20Structure%20%28by%20ref%29))
  (bind _asbp_player (Utilities|Casting|CastToBP_Player OtherActor)
    (:then
      (Default|LoseHealth _asbp_player)
      (Actor|DestroyActor)
      (if (== (Variables|/Game/InfiniteMatrix/Blueprints/BP_Player.BP_Player_C|GetHealth _asbp_player) 0.0)
        (Default|DisplayRestart _asbp_player)))
    (:CastFailed
      (Utilities|Casting|CastToProjectile OtherActor)
      (Actor|DestroyActor)
      (bind _asbp_player_2 (Utilities|Casting|CastToBP_Player (Game|Player|GetPlayerPawn 0)))
      (Default|AddScore _asbp_player_2))))

(event EventBeginPlay)

(event EventTick
  (params (DeltaSeconds :type Float%20%28single-precision%29))
  (Transformation|AddActorLocalRotation (Math|Rotator|MakeRotator (* DeltaSeconds 125.0) 0.0 0.0) false false))

(fn ConstructionScript)